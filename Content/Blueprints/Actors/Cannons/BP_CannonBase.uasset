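; BP_CannonBase is a base cannon actor that fires automatically and repeatedly from BeginPlay.
; After a FireRate delay, it spawns an actor at ProjectileSpawnPoint, scaled by ProjectileScale, then plays CannonFireTimeline from the start.
; The timeline animates the barrel along its relative Y axis, and its Cannon Fire event loops back to the delay to drive the next shot.
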(event `self.ReceiveBeginPlay`
  (`KismetSystemLibrary.Delay` (`self.FireRate`) :!label _label)
  (`self.SpawnProjectile`)
  (bind (_direction _barrellocation) (`Timeline|CannonFireTimeline` :!via `PlayFromStart`)
    (:`Update`
      (`self.Move Cannon Barrel` _barrellocation))
    (:`CannonFire`
      (goto _label))))

(fn `Move Cannon Barrel`
  (params (CannonBarrelYLocation :type "Float (double-precision)"))
  (`SceneComponent.K2_SetRelativeLocation` (`self.Cannon_Barrel`) (`KismetMathLibrary.MakeVector` 0.0 CannonBarrelYLocation) false false))

(fn `SpawnProjectile`
  (bind _projectilespawnpoint (`self.ProjectileSpawnPoint`))
  (`|SpawnActorFromClass` "/Game/Blueprints/Actors/Projectiles/BP_ProjectileBase.BP_ProjectileBase_C" (`KismetMathLibrary.MakeTransform` (`SceneComponent.K2_GetComponentLocation` _projectilespawnpoint) (`SceneComponent.K2_GetComponentRotation` _projectilespawnpoint) (`KismetMathLibrary.Conv_DoubleToVector` (`self.ProjectileScale`))) "AdjustIfPossibleButAlwaysSpawn" "OverrideRootScale" null null))

(fn `UserConstructionScript`)