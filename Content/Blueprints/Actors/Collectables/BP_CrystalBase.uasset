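; BP_CrystalBase is a collectable crystal that flies into the player when touched, then destroys itself.
; On BeginPlay it creates a dynamic instance of the blue crystal material and copies its Color parameter to the crystal's light.
; On player overlap it stores starting values, then a timeline lerps location toward the player's current position while shrinking scale and light intensity to zero.
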(event `self.ReceiveBeginPlay`
  (bind _returnvalue (`PrimitiveComponent.CreateDynamicMaterialInstance` (`self.StaticMesh`) 0 "/Game/Maetrials/MI_Crystal_Blue.MI_Crystal_Blue" "None"))
  (bind _returnvalue_2 (`MaterialInstanceDynamic.K2_GetVectorParameterValue` _returnvalue "Color"))
  (`LightComponent.SetLightColor` (`self.CrystalLight`) _returnvalue_2 true))

(event `self.ReceiveActorBeginOverlap`
  (params (OtherActor :type "Actor Object Reference"))
  (`self.IsPlayer` OtherActor
    (:`IsPlayer`
      (`self.StoreStartingValues`)
      (bind (_direction _collectionprogress _scaleprogress _lightintensityprogress) (`Timeline|Timeline_Collection`)
        (:`Update`
          (`self.MoveToPlayer` _collectionprogress)
          (`self.ScaleCrystal` _scaleprogress)
          (`self.AdjustLightIntensity` _lightintensityprogress))
        (:`Finished`
          (`self.K2_DestroyActor`))))))

(fn `AdjustLightIntensity`
  (params (Alpha :type "Float (double-precision)"))
  (`LightComponent.SetIntensity` (`self.CrystalLight`) (`KismetMathLibrary.Lerp` (`self.StartIntensity`) 0.0 Alpha)))

(fn `MoveToPlayer`
  (params (Alpha :type "Float (double-precision)"))
  (`self.K2_SetActorLocation` (`KismetMathLibrary.VLerp` (`self.StartLocation`) (`self.K2_GetActorLocation` (`GameplayStatics.GetPlayerPawn` 0)) Alpha)))

(fn `ScaleCrystal`
  (params (Alpha :type "Float (double-precision)"))
  (`self.SetActorScale3D` (`KismetMathLibrary.VLerp` (`self.StartScale`) (0.0 0.0 0.0) Alpha)))

(fn `StoreStartingValues`
  (set `self.StartLocation` (`self.K2_GetActorLocation`))
  (set `self.StartScale` (`self.GetActorScale3D`))
  (set `self.StartIntensity` (`LightComponentBase.Intensity` (`self.CrystalLight`))))

(fn `UserConstructionScript`)